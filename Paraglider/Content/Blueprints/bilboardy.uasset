(event `self.ReceiveBeginPlay`
  (bind _textfields (`self.TextFields`))
  (bind _ashigh_score_editable_line (cast `/Game/FirstPersonBP/Blueprints/HighScoreEditableLine` (`ChildActorComponent.ChildActor` (`self.TextField1`))))
  (`KismetArrayLibrary.Array_Add` _textfields _ashigh_score_editable_line)
  (bind _ashigh_score_editable_line_2 (cast `/Game/FirstPersonBP/Blueprints/HighScoreEditableLine` (`ChildActorComponent.ChildActor` (`self.TextField2`))))
  (`KismetArrayLibrary.Array_Add` _textfields _ashigh_score_editable_line_2)
  (bind _ashigh_score_editable_line_3 (cast `/Game/FirstPersonBP/Blueprints/HighScoreEditableLine` (`ChildActorComponent.ChildActor` (`self.TextField3`))))
  (`KismetArrayLibrary.Array_Add` _textfields _ashigh_score_editable_line_3)
  (bind _ashigh_score_editable_line_4 (cast `/Game/FirstPersonBP/Blueprints/HighScoreEditableLine` (`ChildActorComponent.ChildActor` (`self.TextField4`))))
  (`KismetArrayLibrary.Array_Add` _textfields _ashigh_score_editable_line_4)
  (bind _ashigh_score_editable_line_5 (cast `/Game/FirstPersonBP/Blueprints/HighScoreEditableLine` (`ChildActorComponent.ChildActor` (`self.TextField5`))))
  (`KismetArrayLibrary.Array_Add` _textfields _ashigh_score_editable_line_5)
  (`SceneComponent.SetVisibility` (`self.TextHighScoresTitle`) false false)
  (`PrimitiveComponent.SetMaterial` (`self.StaticMesh6`) 2 "/Game/Materials/screen.screen")
  (for (_array_element _array_index) (`self.TextFields`)
    (`/Game/FirstPersonBP/Blueprints/HighScoreEditableLine.EventSetNumber` _array_element (+ _array_index 1))
    (`/Game/FirstPersonBP/Blueprints/HighScoreEditableLine.EventSetEditable` _array_element false)
    (`/Game/FirstPersonBP/Blueprints/HighScoreEditableLine.EventSetEnabled` _array_element false)
    (bind _ashigh_score_editable_line_6 (cast `/Game/FirstPersonBP/Blueprints/HighScoreEditableLine` (`ChildActorComponent.ChildActor` (`self.TextFieldYou`))))
    (`/Game/FirstPersonBP/Blueprints/HighScoreEditableLine.EventSetEnabled` _ashigh_score_editable_line_6 false)))

(event `self.ReceiveActorBeginOverlap`
  (params (OtherActor :type "Actor Object Reference")))

(event `self.ReceiveTick`
  (params (DeltaSeconds :type "Float (single-precision)")))

(event `DisplayHighScores`
  (params (PointArray :type "Array of Integer (by ref)") (NameArray :type "Array of String (by ref)") (AllowInputNewHighScore :type Boolean))
  (bind _returnvalue (- (`KismetMathLibrary.Min` (`KismetArrayLibrary.Array_Length` PointArray) (`KismetArrayLibrary.Array_Length` NameArray) 5) -1))
  (`SceneComponent.SetVisibility` (`self.TextHighScoresTitle`) true false)
  (`PrimitiveComponent.SetMaterial` (`self.StaticMesh6`) 2 "/Game/Materials/ScreeGlow_mat.ScreeGlow_mat")
  (for (_array_element _array_index) (`self.TextFields`)
    (`/Game/FirstPersonBP/Blueprints/HighScoreEditableLine.EventSetEnabled` _array_element true)
    (`/Game/FirstPersonBP/Blueprints/HighScoreEditableLine.EventSetNameAndScore` _array_element (`KismetArrayLibrary.Array_Get` NameArray (`KismetMathLibrary.Min` _array_index _returnvalue)) (`KismetArrayLibrary.Array_Get` PointArray (`KismetMathLibrary.Min` _array_index _returnvalue)))
    (if AllowInputNewHighScore
      (bind _ashigh_score_editable_line (cast `/Game/FirstPersonBP/Blueprints/HighScoreEditableLine` (`ChildActorComponent.ChildActor` (`self.TextFieldYou`))))
      (`/Game/FirstPersonBP/Blueprints/HighScoreEditableLine.EventSetEnabled` _ashigh_score_editable_line true)
      (`/Game/FirstPersonBP/Blueprints/HighScoreEditableLine.EventSetEditable` _ashigh_score_editable_line true)
      (bind _asplayer_controller (cast `PlayerController` (`Pawn.GetController` (`self.Player`))))
      (`self.EnableInput` _ashigh_score_editable_line _asplayer_controller)
      (else
        (bind _ashigh_score_editable_line_2 (cast `/Game/FirstPersonBP/Blueprints/HighScoreEditableLine` (`ChildActorComponent.ChildActor` (`self.TextFieldYou`))))
        (`/Game/FirstPersonBP/Blueprints/HighScoreEditableLine.EventSetEnabled` _ashigh_score_editable_line_2 false)
        (`/Game/FirstPersonBP/Blueprints/HighScoreEditableLine.EventSetEditable` _ashigh_score_editable_line_2 false)))))

(fn `SetFreezerVisibility`
  (params (Visibility :type Boolean))
  (`SceneComponent.SetVisibility` (`self.ColaFreezer`) Visibility false))

(fn `UserConstructionScript`)